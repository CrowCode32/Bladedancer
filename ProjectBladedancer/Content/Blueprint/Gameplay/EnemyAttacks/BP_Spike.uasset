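; BP_Spike is an enemy attack Blueprint that raises a spike sprite when the attack starts.
; StartAttack runs the parent logic, then fires RaiseSpikes, which plays a timeline.
; Each timeline update lerps the sprite's world Z from StartLocation to EndLocation by the Progress track, keeping X and Y at StartLocation.
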(event Custom|RaiseSpikes
  (bind _startlocation (Variables|Default|GetStartLocation))
  (bind _progress (Timeline|Timeline Play)
    (:Update
      (Transformation|SetWorldLocation (Variables|Default|GetSprite) (Math|Vector|MakeVector (.x (.location _startlocation)) (.y (.location _startlocation)) (Math|Float|Lerp (.z (.location _startlocation)) (.z (.location (Variables|Default|GetEndLocation))) _progress)) false false))))

(event EventBeginPlay
  (|CallParentFunction))

(fn ConstructionScript
  (|CallParentFunction))

(fn StartAttack
  (|CallParentFunction)
  (CallFunction|RaiseSpikes))