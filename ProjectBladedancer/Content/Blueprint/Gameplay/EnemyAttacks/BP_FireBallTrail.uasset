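; Enemy fireball attack that, when started, arcs away to a randomized point and then swoops at the player.
; BeginPlay picks that point from a random world X/Z offset off the parent's start location.
; Two chained timelines lerp the position with a sine height offset, bowing upward on the way out and downward on the attack.
; The player's location is sampled once between arcs, so the fireball does not home.
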(event Custom|Movement
  (bind _progress (Timeline|ArcAway Play)
    (:Update
      (Transformation|SetActorLocation (+ (.location (Math|Transform|Lerp(Transform) (Variables|Default|GetStartLocation) (Variables|Default|GetPauseLocation) _progress)) (* "0.000000,0.000000,1.000000" (Variables|Default|GetArcHeight) (Math|Trig|Sin(Degrees) (* _progress 1.8e+02)))) false false))
    (:Finished
      (Variables|Default|SetPlayerLocation (Transformation|GetActorTransform (Game|GetPlayerCharacter 0)))
      (bind _progress_2 (Timeline|ArcTowardsPlayer Play)
        (:Update
          (Transformation|SetActorLocation (+ (.location (Math|Transform|Lerp(Transform) (Variables|Default|GetPauseLocation) (Variables|Default|GetPlayerLocation) _progress_2)) (* "0.000000,0.000000,-1.000000" (Variables|Default|GetArcHeight) (Math|Trig|Sin(Degrees) (* _progress_2 1.8e+02)))) false false))))))

(event EventBeginPlay
  (|CallParentFunction)
  (Variables|Default|SetPauseLocation (Math|Conversions|ToTransform(Vector) (+ (Math|Vector|MakeVector (Math|Random|RandomFloatinRange -6e+02 -2e+02) 0.0 (Math|Random|RandomFloatinRange 2e+02 5e+02)) (.location (Variables|Default|GetStartLocation))))))

(fn ConstructionScript
  (|CallParentFunction))

(fn StartAttack
  (|CallParentFunction)
  (CallFunction|Movement))