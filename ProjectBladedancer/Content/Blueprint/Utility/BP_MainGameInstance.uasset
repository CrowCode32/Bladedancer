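; Main game instance that acts as a central entry point for dialogue and cutscene control, forwarding calls to DialogueManager and CutsceneManager.
; Dialogue starts by row name, and progressing either advances a completed line or skips its typing.
; Playing a cutscene binds an event to dialogue completion, then plays the fixed LS_Start sequence.
; Separate pause and resume calls let the cutscene halt and continue.
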(event Custom|ResumeCutscene
  (Class|CutsceneManager|ContinueCutscene (Subsystems|GetCutsceneManager)))

(fn GIStartDialogue
  (params (RowName :type Name))
  (Class|DialogueManager|StartDialogue (Subsystems|GetDialogueManager) RowName))

(fn GIProgressDialogue
  (bind _returnvalue (Class|DialogueManager|GetLineComplete (Subsystems|GetDialogueManager)))
  (if _returnvalue
    (Class|DialogueManager|ProgressDialogue (Subsystems|GetDialogueManager))
    (else
      (Class|DialogueManager|SkipTyping (Subsystems|GetDialogueManager)))))

(fn GIPlayCutscene
  (EventDispatchers|BindEventtoDialogueComplete (Subsystems|GetDialogueManager) (EventDispatchers|CreateEvent :!event Custom|ResumeCutscene))
  (Class|CutsceneManager|PlayCutscene (Subsystems|GetCutsceneManager) "/Game/Cinematics/LS_Start.LS_Start"))

(fn GIPauseCutscene
  (Class|CutsceneManager|PauseCutscene (Subsystems|GetCutsceneManager)))