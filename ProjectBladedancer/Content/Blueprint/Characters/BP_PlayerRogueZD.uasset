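; BP_PlayerRogueZD is the player Rogue character, with side-scroller style movement along the world X axis and jumping.
; On BeginPlay it caches its PlayerController, creates and displays the WBP_PlayerHUD widget, then adds the movement and interact Enhanced Input mapping contexts.
; Movement and jump inputs drive the built-in character functions, while completing the interact input tells BP_MainGameInstance to progress dialogue.
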(event Input|EnhancedActionEvents|EnhancedInputActionIA_Movement
  (params (ActionValue :type Vector%202D%20Structure) (ElapsedSeconds :type Float%20%28double-precision%29) (TriggeredSeconds :type Float%20%28double-precision%29) (InputAction :type Input%20Action%20Object%20Reference :default "/Game/Blueprint/Gameplay/Input/IA_Movement.IA_Movement"))
  (Pawn|Input|AddMovementInput "1.000000,0.000000,0.000000" (.X (Math|Vector2D|BreakVector2D ActionValue)) false))

(event Input|EnhancedActionEvents|EnhancedInputActionIA_Jump
  (params (ActionValue :type Boolean) (ElapsedSeconds :type Float%20%28double-precision%29) (TriggeredSeconds :type Float%20%28double-precision%29) (InputAction :type Input%20Action%20Object%20Reference :default "/Game/Blueprint/Gameplay/Input/IA_Jump.IA_Jump"))
  (:Started
    (Character|Jump)))

(event Input|EnhancedActionEvents|EnhancedInputActionIA_Interact
  (params (ActionValue :type Boolean) (ElapsedSeconds :type Float%20%28double-precision%29) (TriggeredSeconds :type Float%20%28double-precision%29) (InputAction :type Input%20Action%20Object%20Reference :default "/Game/Blueprint/Gameplay/Input/IA_Interact.IA_Interact"))
  (:Completed
    (bind _asbp_main_game_instance (Utilities|Casting|CastToBP_MainGameInstance (Game|GetGameInstance)))
    (Default|GIProgressDialogue _asbp_main_game_instance)))

(event EventBeginPlay
  (bind _returnvalue (Game|GetPlayerController 0))
  (bind _returnvalue_2 (PlayerController|LocalPlayerSubsystems|GetEnhancedInputLocalPlayerSubsystem _returnvalue))
  (bind _asplayer_controller (Utilities|Casting|CastToPlayerController (Pawn|GetController)))
  (Variables|Default|SetPlayerController _asplayer_controller)
  ;[0.15 0.15 0.15 0.5] HUD
  (bind _returnvalue_3 (UserInterface|CreateWidget (Variables|Default|GetHUDClass) (Variables|Default|GetPlayerController)))
  (bind _aswbp_player_hud (Utilities|Casting|CastToWBP_PlayerHUD _returnvalue_3))
  (bind _output_get (Variables|Default|SetPlayerHUD _aswbp_player_hud))
  (UserInterface|Viewport|AddtoViewport _output_get 0)
  ;[0.15 0.15 0.15 0.5] Input
  (Input|AddMappingContext _returnvalue_2 "/Game/Blueprint/Gameplay/Input/IMC_Movement.IMC_Movement" 0 "(bIgnoreAllPressedKeysUntilRelease=True,bForceImmediately=False,bNotifyUserSettings=False)")
  (Input|AddMappingContext _returnvalue_2 "/Game/Blueprint/Gameplay/Input/IMC_Interact.IMC_Interact" 0 "(bIgnoreAllPressedKeysUntilRelease=True,bForceImmediately=False,bNotifyUserSettings=False)"))

(fn ConstructionScript
  (|CallParentFunction))